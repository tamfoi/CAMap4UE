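; AC_MapGenerator is a map generator component that builds a Width by Height tile grid.
; GenerateMap calls InitializeMap, which clears and resizes Map as an array of row structs, each holding a List of tiles.
; Its nested loop detects outer-edge cells meant to become walls, but that branch is still empty.
; SetTile writes a tile at X, Y through row-then-column indexing, though nothing here calls it yet.
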(event `GenerateMap`
  (`self.InitializeMap`))

(fn `InitializeMap`
  (locals (RowIndex :type Integer) (ColumnIndex :type Integer))
  ;[1 1 1] 配列の初期化
  (`KismetArrayLibrary.Array_Clear` (`self.Map`))
  (`KismetArrayLibrary.Array_Resize` (`self.Map`) (`self.Height`))
  (for (_array_element _array_index) (`self.Map`)
    (set `local.RowIndex` _array_index)
    (if (`KismetArrayLibrary.Array_IsEmpty` (break `/Game/CAMap4UE/Blueprints/F_MapColumn` _array_element))
      (`KismetArrayLibrary.Array_Resize` (break `/Game/CAMap4UE/Blueprints/F_MapColumn` _array_element) (`self.Width`)))
    (for (_ _array_index_2) (break `/Game/CAMap4UE/Blueprints/F_MapColumn` _array_element)
      (set `local.ColumnIndex` _array_index_2)
      ;[1 1 1] 外周は壁
      (if (or (== (`local.ColumnIndex`) 0) (== (`local.RowIndex`) 0) (== (`local.ColumnIndex`) (- (`self.Width`) 1)) (== (`local.RowIndex`) (- (`self.Height`) 1)))
        _))))

(fn `SetTile`
  (params (X :type Integer) (Y :type Integer) (Tile :type "/Game/CAMap4UE/Blueprints/E_MapTile Enum" :default "NewEnumerator0"))
  (bind _output_list (break `/Game/CAMap4UE/Blueprints/F_MapColumn` (`|GetArrayItem` (`self.Map`) Y)))
  (`KismetArrayLibrary.Array_Set` _output_list X Tile))